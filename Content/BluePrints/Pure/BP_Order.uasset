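; BP_Order runs the command game loop, issuing random bark, jump, run or running-jump orders to the player's BP_Wolf.
; Tick checks the wolf's action flags, scoring a match and scheduling the next order.
; A named CheckComplete timer, shortened each order down to a minimum, fails late orders and removes a heart.
; Losing the last heart opens the game-over widget with the score and a conditional best-score label.
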(event `self.ReceiveBeginPlay`
  (`self.GetWolf`)
  (`self.GetOrderWidget`)
  (`self.OrderStart`))

(event `self.ReceiveTick`
  (params (DeltaSeconds :type "Float (single-precision)"))
  (`self.OrderCourse` (`self.OrderNum`)))

(fn `CheckComplete`
  (set `self.IsStart` false)
  (set `self.IsComplete` false)
  (`self.FailOrder`)
  (`self.HeartDecrease`)
  (if (not (`self.IsGameOver`))
    (`KismetSystemLibrary.K2_SetTimer` null "OrderStart" (`self.OrderInterval`))))

(fn `GameOver`
  (locals (WG_GameOver :type "/Game/BluePrints/Widget/WGBP_GameOver Object Reference"))
  (bind _besttext (`/Game/BluePrints/Widget/WGBP_GameOver.BestText` (`local.WG_GameOver`)))
  (`GameplayStatics.PlaySound2D` "/Game/Resources/Sounds/SFX/Game_Over_Cue.Game_Over_Cue" 1.0 1.0 0.0 null null)
  (set `self.IsGameOver` true)
  (bind _returnvalue (`|CreateWidget` "/Game/BluePrints/Widget/WGBP_GameOver.WGBP_GameOver_C" (`GameplayStatics.GetPlayerController` 0)))
  (bind _output_get (set `local.WG_GameOver` _returnvalue))
  (`UserWidget.AddToViewport` _output_get 0)
  (`TextBlock.SetText` (`/Game/BluePrints/Widget/WGBP_GameOver.ScoreText` (`local.WG_GameOver`)) (`KismetTextLibrary.Conv_IntToText` (`self.Score`)))
  (bind _returnvalue_2 (`self.CompareScore` (`self.Score`)))
  (if _returnvalue_2
    (`Widget.SetVisibility` _besttext "Visible")
    (else
      (`Widget.SetVisibility` _besttext "Hidden"))))

(fn `GetWolf`
  (bind _asbp_wolf (cast `/Game/BluePrints/Pure/BP_Wolf` (`GameplayStatics.GetPlayerPawn` 0)))
  (set `self.Wolf` _asbp_wolf))

(fn `HeartDecrease`
  (locals (OrderWidget :type "/Game/BluePrints/Widget/WGBP_Order Object Reference"))
  (`GameplayStatics.PlaySound2D` "/Game/Resources/Sounds/SFX/Heart_Decrease_Cue.Heart_Decrease_Cue" 1.0 1.0 0.0 null null)
  (`/Engine/EditorBlueprintResources/StandardMacros.DecrementInt` (`self.HeartNum`)
    (:`  `
      (bind _foundwidgets (`WidgetBlueprintLibrary.GetAllWidgetsOfClass` "/Game/BluePrints/Widget/WGBP_Order.WGBP_Order_C"))
      (bind _aswgbp_order (cast `/Game/BluePrints/Widget/WGBP_Order` (`|GetArrayItem` _foundwidgets)))
      (set `local.OrderWidget` _aswgbp_order)
      (switch `int` (`self.HeartNum`)
        (:`0`
          (set `Widget.Visibility` "Hidden" (`/Game/BluePrints/Widget/WGBP_Order.Heart3` (`local.OrderWidget`)))
          (`self.GameOver`))
        (:`1`
          (set `Widget.Visibility` "Hidden" (`/Game/BluePrints/Widget/WGBP_Order.Heart2` (`local.OrderWidget`))))
        (:`2`
          (set `Widget.Visibility` "Hidden" (`/Game/BluePrints/Widget/WGBP_Order.Heart1` (`local.OrderWidget`))))))))

(fn `OrderCourse`
  (params (OrderNum :type Integer))
  (bind _wolf (`self.Wolf`))
  (if (`self.IsStart`)
    (switch `int` OrderNum
      (:`0`
        (`self.OrderReuslt` (`/Game/BluePrints/Pure/BP_Wolf.IsBarkCheck` (`self.Wolf`))))
      (:`1`
        (`self.OrderReuslt` (`/Game/BluePrints/Pure/BP_Wolf.IsJumpCheck` (`self.Wolf`))))
      (:`2`
        (`self.OrderReuslt` (`/Game/BluePrints/Pure/BP_Wolf.IsRunningCheck` (`self.Wolf`))))
      (:`3`
        (`self.OrderReuslt` (and (`/Game/BluePrints/Pure/BP_Wolf.IsRunningCheck` _wolf) (`/Game/BluePrints/Pure/BP_Wolf.IsJumpCheck` _wolf)))))))

(fn `OrderReuslt`
  (params (Order :type Boolean))
  (bind _output_get (set `self.IsComplete` Order))
  (if _output_get
    (set `self.IsStart` false)
    (`KismetSystemLibrary.K2_ClearTimer` null "CheckComplete")
    (`self.CompleteOrder`)
    (`/Engine/EditorBlueprintResources/StandardMacros.IncrementInt` (`self.Score`)
      (:`  `
        (`KismetSystemLibrary.K2_SetTimer` null "OrderStart" (`self.OrderInterval`))))))

(fn `OrderStart`
  (`GameplayStatics.PlaySound2D` "/Game/Resources/Sounds/SFX/Order_Cue.Order_Cue" 1.0 1.0 0.0 null null)
  (`/Game/BluePrints/Pure/BP_Wolf.InitBool` (`self.Wolf`))
  (bind _returnvalue (`self.RandomOrder`))
  (set `self.OrderNum` _returnvalue)
  (set `self.IsStart` true)
  (bind _output_get (set `self.OrderDelay` (- (`self.OrderDelay`) (`self.DecreaseOrderDelay`))))
  (if (> _output_get (`self.OrderDelayMin`))
    (bind _output_get_2 (set `self.OrderDelay` (`self.OrderDelay`)))
    (`KismetSystemLibrary.K2_SetTimer` null "CheckComplete" _output_get_2)
    (else
      (bind _output_get_3 (set `self.OrderDelay` (`self.OrderDelayMin`)))
      (`KismetSystemLibrary.K2_SetTimer` null "CheckComplete" _output_get_3))))

(fn `UserConstructionScript`)